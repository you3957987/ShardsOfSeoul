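; BP_Direction is a proximity-triggered direction guide in the cable car map that shows Niagara arrows to the player.
; The arrows are deactivated at BeginPlay unless AutoActivate is set; Sphere overlaps with actors tagged Player switch them on and off.
; Entering also enables custom depth with a stencil value on the static meshes of the referenced CustomDepth actor, which is not reverted on exit.
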(event `self.ReceiveBeginPlay`
  (if (not (`self.AutoActivate`))
    (`ActorComponent.Deactivate` (`self.NS_Direction_Arrows_04`))))

(event `self.Sphere.OnComponentBeginOverlap`
  (params (OverlappedComponent :type "PrimitiveComponent Object Reference") (OtherActor :type "Actor Object Reference") (OtherComp :type "PrimitiveComponent Object Reference") (OtherBodyIndex :type Integer) (bFromSweep :type Boolean) (SweepResult :type "HitResult Structure (by ref)"))
  (if (`self.ActorHasTag` OtherActor "Player")
    (`ActorComponent.Activate` (`self.NS_Direction_Arrows_04`) false)
    (`/Engine/EditorBlueprintResources/StandardMacros.IsValid` (`self.CustomDepth`)
      (:`Is Valid`
        (for _array_element (`self.K2_GetComponentsByClass` (`self.CustomDepth`) "/Script/Engine.StaticMeshComponent")
          (`PrimitiveComponent.SetRenderCustomDepth` _array_element true)
          (`PrimitiveComponent.SetCustomDepthStencilValue` _array_element 2))))))

(event `self.Sphere.OnComponentEndOverlap`
  (params (OverlappedComponent :type "PrimitiveComponent Object Reference") (OtherActor :type "Actor Object Reference") (OtherComp :type "PrimitiveComponent Object Reference") (OtherBodyIndex :type Integer))
  (if (`self.ActorHasTag` OtherActor "Player")
    (`ActorComponent.Deactivate` (`self.NS_Direction_Arrows_04`))))

(fn `UserConstructionScript`)
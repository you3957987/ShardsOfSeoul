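; BP_Elevator is a lift in the cable car map that carries the player character upward, then returns empty.
; Box overlap by the player disables input and the box's collision, attaches the character to Cube, and blends the view to the elevator.
; A timeline raises Cube; on finish the character detaches with input restored, a tiny launch, and control rotation matched to Camera.
; A second timeline lowers Cube, then re-enables the trigger.
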(event `self.Box.OnComponentBeginOverlap`
  (params (OverlappedComponent :type "PrimitiveComponent Object Reference") (OtherActor :type "Actor Object Reference") (OtherComp :type "PrimitiveComponent Object Reference") (OtherBodyIndex :type Integer) (bFromSweep :type Boolean) (SweepResult :type "HitResult Structure (by ref)"))
  (if (== OtherActor (`GameplayStatics.GetPlayerPawn` 0))
    (bind `_as캐릭터` (cast `Character` OtherActor))
    (bind _output_get (set `self.Character` `_as캐릭터`))
    (`self.DisableInput` _output_get (`GameplayStatics.GetPlayerController` 0))
    (`PrimitiveComponent.SetCollisionEnabled` (`self.Box`) "NoCollision")
    (`self.K2_AttachToComponent` _output_get (`self.Cube`) "None" "KeepWorld" "KeepWorld" "KeepWorld" true)
    (`self.ImpulseElevator`)
    (`PlayerController.SetViewTargetWithBlend` (`GameplayStatics.GetPlayerController` 0) self 1.0 "VTBlend_Linear" 0.0 false)))

(event `ImpulseElevator`
  (bind _returnvalue (`GameplayStatics.GetPlayerController` 0))
  (bind _character (`self.Character`))
  (bind (_direction _up) (`Timeline|AddImpuleElevator` :!via `PlayFromStart`)
    (:`Update`
      (`SceneComponent.K2_SetRelativeLocation` (`self.Cube`) (`KismetMathLibrary.MakeVector` 0.0 0.0 (`KismetMathLibrary.Lerp` 0.0 1800.0 _up)) false false))
    (:`Finished`
      (`self.K2_DetachFromActor` (`self.Character`) "KeepWorld" "KeepWorld" "KeepWorld")
      (`self.EnableInput` _character (`GameplayStatics.GetPlayerController` 0))
      (`Character.LaunchCharacter` _character (0.0 0.0 0.1) false false)
      (`PlayerController.SetViewTargetWithBlend` _returnvalue (`self.Character`) 0.1 "VTBlend_Linear" 0.0 false)
      (`Controller.SetControlRotation` _returnvalue (`SceneComponent.K2_GetComponentRotation` (`self.Camera`)))
      (bind (_direction_2 `_새_트랙_0`) (`Timeline|타임라인` :!via `PlayFromStart`)
        (:`Update`
          (`SceneComponent.K2_SetRelativeLocation` (`self.Cube`) (`KismetMathLibrary.MakeVector` 0.0 0.0 (`KismetMathLibrary.Lerp` 1800.0 0.0 `_새_트랙_0`)) false false))
        (:`Finished`
          (`PrimitiveComponent.SetCollisionEnabled` (`self.Box`) "QueryAndPhysics"))))))

(fn `UserConstructionScript`)
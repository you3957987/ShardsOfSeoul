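; BP_AutoTowerCrane is a tower crane that starts rotating automatically after taking repeated hits.
; Each damage event counts on itself and LinkedCrane, raising a white progress parameter on a dynamic overlay material shared by its static meshes.
; At the hit threshold, a timeline animates the overlay, then custom-depth stencil is enabled and tags are cleared.
; A timer then loops a rotation timeline with audio, alternating direction after each swing.
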(event `self.ReceiveBeginPlay`
  (add `self.OnTakeAnyDamage` (delegate `OnTakeAnyDamage_Event`))
  (bind _returnvalue (`KismetMaterialLibrary.CreateDynamicMaterialInstance` "/Game/CableCarMap/Material/M_WhiteOverlay.M_WhiteOverlay"))
  (set `self.OverlayMID` _returnvalue)
  (for _array_element (`self.K2_GetComponentsByClass` "/Script/Engine.StaticMeshComponent")
    (`MeshComponent.SetOverlayMaterial` _array_element (`self.OverlayMID`))))

(event `OnTakeAnyDamage_Event` :!signature `self.OnTakeAnyDamage`
  (params (DamagedActor :type "Actor Object Reference") (Damage :type "Float (single-precision)") (DamageType :type "DamageType Object Reference") (InstigatedBy :type "Controller Object Reference") (DamageCauser :type "Actor Object Reference"))
  (`self.CountDown` (`self.LinkedCrane`))
  (`self.CountDown`))

(event `CountDown`
  (bind _count (`self.Count`))
  (`/Engine/EditorBlueprintResources/StandardMacros.IncrementInt` _count
    (:`  `
      (`MaterialInstanceDynamic.SetScalarParameterValue` (`self.OverlayMID`) "WhiteProgress" (`KismetMathLibrary.Square` (/ (`KismetMathLibrary.Conv_IntToDouble` _count) 100.0)))
      (if (>= (`self.Count`) 10)
        (bind (_direction `_새_트랙_0`) (`Timeline|타임라인_0` :!via `PlayFromStart`)
          (:`Update`
            (`MaterialInstanceDynamic.SetScalarParameterValue` (`self.OverlayMID`) "WhiteProgress" `_새_트랙_0`))
          (:`Finished`
            (for _array_element (`self.K2_GetComponentsByClass` "/Script/Engine.StaticMeshComponent")
              (`PrimitiveComponent.SetRenderCustomDepth` _array_element true)
              (`PrimitiveComponent.SetCustomDepthStencilValue` _array_element 2))
            (`KismetArrayLibrary.Array_Clear` (`self.Tags`))
            (`KismetSystemLibrary.K2_SetTimerDelegate` (delegate `ActiveCrane`) 2.0 :!label _label)))))))

(event `ActiveCrane`
  (`AudioComponent.Play` (`self.Audio`) 0.0)
  (if (`self.reverse`)
    (bind (_direction _rotation) (`Timeline|타임라인` :!via `ReverseFromEnd` :!label _label_2)
      (:`Update`
        (`SceneComponent.K2_SetRelativeRotation` (`self.SM_Props_TowerCrane_02_2`) (`KismetMathLibrary.MakeRotator` 0.0 0.0 (* _rotation (`self.minus`))) false false))
      (:`Finished`
        (set `self.reverse` (not (`self.reverse`)))
        (goto _label)))
    (else
      (goto _label_2 :!via `PlayFromStart`))))

(fn `UserConstructionScript`)
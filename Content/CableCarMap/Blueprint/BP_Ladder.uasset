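; BP_Ladder is a climbable ladder for the player character in the cable car map.
; When the player pawn enters the Floor overlap volume, it stores the ShardsOfSeoulCharacter, switches its movement to Flying and sets its climbing flag.
; A high flying braking deceleration is applied during the climb.
; Leaving the volume restores Walking, clears the flag and resets the braking to zero.
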(event `self.Floor.OnComponentBeginOverlap`
  (params (OverlappedComponent :type "PrimitiveComponent Object Reference") (OtherActor :type "Actor Object Reference") (OtherComp :type "PrimitiveComponent Object Reference") (OtherBodyIndex :type Integer) (bFromSweep :type Boolean) (SweepResult :type "HitResult Structure (by ref)"))
  (if (== OtherActor (`GameplayStatics.GetPlayerPawn` 0))
    (bind _asshards_of_seoul_character (cast `ShardsOfSeoulCharacter` OtherActor))
    (bind _output_get (set `self.Character` _asshards_of_seoul_character))
    (bind _charactermovement (`Character.CharacterMovement` _output_get))
    (`CharacterMovementComponent.SetMovementMode` _charactermovement "MOVE_Flying" 0)
    (`ShardsOfSeoulCharacter.SetIsClimbing` _output_get true)
    (set `CharacterMovementComponent.BrakingDecelerationFlying` 4000.0 _charactermovement)))

(event `self.Floor.OnComponentEndOverlap`
  (params (OverlappedComponent :type "PrimitiveComponent Object Reference") (OtherActor :type "Actor Object Reference") (OtherComp :type "PrimitiveComponent Object Reference") (OtherBodyIndex :type Integer))
  (bind _character (`self.Character`))
  (bind _charactermovement (`Character.CharacterMovement` _character))
  (if (== OtherActor (`self.Character`))
    (`CharacterMovementComponent.SetMovementMode` _charactermovement "MOVE_Walking" 0)
    (`ShardsOfSeoulCharacter.SetIsClimbing` _character false)
    (set `CharacterMovementComponent.BrakingDecelerationFlying` 0.0 _charactermovement)))

(fn `UserConstructionScript`)
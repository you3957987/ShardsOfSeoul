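; BP_CameraZoomOut is a trigger box actor that changes camera zoom, by its name a zoom out, for characters passing through it.
; Begin overlap stores the Character and plays a timeline that lerps its SpringArm length between TargetArmLength and ArmLength.
; End overlap by that stored Character plays a second timeline with the same lerp inputs, its own curve setting the direction.
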(event `self.Box.OnComponentBeginOverlap`
  (params (OverlappedComponent :type "PrimitiveComponent Object Reference") (OtherActor :type "Actor Object Reference") (OtherComp :type "PrimitiveComponent Object Reference") (OtherBodyIndex :type Integer) (bFromSweep :type Boolean) (SweepResult :type "HitResult Structure (by ref)"))
  (bind `_as캐릭터` (cast `Character` OtherActor))
  (bind _output_get (set `self.As캐릭터` `_as캐릭터`))
  (bind _returnvalue (`self.GetComponentByClass` _output_get "/Script/Engine.SpringArmComponent"))
  (`/Engine/EditorBlueprintResources/StandardMacros.IsValid` _returnvalue
    (:`Is Valid`
      (bind (_direction `_새_트랙_0`) (`Timeline|타임라인` :!via `PlayFromStart`)
        (:`Update`
          (set `SpringArmComponent.TargetArmLength` (`KismetMathLibrary.Lerp` (`self.Target Arm Length`) (`self.ArmLength`) `_새_트랙_0`) _returnvalue))))))

(event `self.Box.OnComponentEndOverlap`
  (params (OverlappedComponent :type "PrimitiveComponent Object Reference") (OtherActor :type "Actor Object Reference") (OtherComp :type "PrimitiveComponent Object Reference") (OtherBodyIndex :type Integer))
  (bind `_as캐릭터` (`self.As캐릭터`))
  (bind _returnvalue (`self.GetComponentByClass` `_as캐릭터` "/Script/Engine.SpringArmComponent"))
  (if (== OtherActor `_as캐릭터`)
    (`/Engine/EditorBlueprintResources/StandardMacros.IsValid` _returnvalue
      (:`Is Valid`
        (bind (_direction `_새_트랙_0`) (`Timeline|타임라인_0` :!via `PlayFromStart`)
          (:`Update`
            (set `SpringArmComponent.TargetArmLength` (`KismetMathLibrary.Lerp` (`self.Target Arm Length`) (`self.ArmLength`) `_새_트랙_0`) _returnvalue)))))))

(fn `UserConstructionScript`)
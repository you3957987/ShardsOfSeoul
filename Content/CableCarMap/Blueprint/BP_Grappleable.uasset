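; BP_Grappleable is an actor that serves as a grapple target for the player character.
; When a ShardsOfSeoulCharacter enters its Sphere1 trigger, it caches that character and registers itself with the character's GrappleComp.
; When the cached character leaves the sphere, it unregisters itself and clears the reference.
; Only one character reference is held at a time, and the actor does no per-frame work.
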(event `self.Sphere1.OnComponentBeginOverlap`
  (params (OverlappedComponent :type "PrimitiveComponent Object Reference") (OtherActor :type "Actor Object Reference") (OtherComp :type "PrimitiveComponent Object Reference") (OtherBodyIndex :type Integer) (bFromSweep :type Boolean) (SweepResult :type "HitResult Structure (by ref)"))
  (bind _asshards_of_seoul_character (cast `ShardsOfSeoulCharacter` OtherActor))
  (bind _output_get (set `self.As Shards Of Seoul Character` _asshards_of_seoul_character))
  (`GrappleComp.AddGrappleTarget` (`ShardsOfSeoulCharacter.GrappleComp` _output_get) self))

(event `self.Sphere1.OnComponentEndOverlap`
  (params (OverlappedComponent :type "PrimitiveComponent Object Reference") (OtherActor :type "Actor Object Reference") (OtherComp :type "PrimitiveComponent Object Reference") (OtherBodyIndex :type Integer))
  (bind _as_shards_of_seoul_character (`self.As Shards Of Seoul Character`))
  (if (== OtherActor _as_shards_of_seoul_character)
    (`GrappleComp.RemoveGrappleTarget` (`ShardsOfSeoulCharacter.GrappleComp` _as_shards_of_seoul_character) self)
    (set `self.As Shards Of Seoul Character` null)))

(fn `UserConstructionScript`)
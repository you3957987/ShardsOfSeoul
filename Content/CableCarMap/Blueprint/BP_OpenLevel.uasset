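; BP_OpenLevel is a trigger actor that plays a short transition and moves the player to the TopOfNamsan level.
; When an actor tagged Player overlaps its Box, it disables player input and blends the view to itself.
; As the blend nears its end, the camera fades out and holds, then the level opens by name after timed delays.
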(event `self.Box.OnComponentBeginOverlap`
  (params (OverlappedComponent :type "PrimitiveComponent Object Reference") (OtherActor :type "Actor Object Reference") (OtherComp :type "PrimitiveComponent Object Reference") (OtherBodyIndex :type Integer) (bFromSweep :type Boolean) (SweepResult :type "HitResult Structure (by ref)"))
  (bind _returnvalue (`GameplayStatics.GetPlayerController` 0))
  (if (`self.ActorHasTag` OtherActor "Player")
    (`self.DisableInput` (`GameplayStatics.GetPlayerPawn` 0) _returnvalue)
    (`PlayerController.SetViewTargetWithBlend` _returnvalue self 5.0 "VTBlend_Linear" 0.0 false)
    (`KismetSystemLibrary.Delay` 4.0)
    (`PlayerCameraManager.StartCameraFade` :`self` (`PlayerController.PlayerCameraManager` _returnvalue) :`ToAlpha` 1.0 :`Duration` 1.0 :`bHoldWhenFinished` true)
    (`KismetSystemLibrary.Delay` 1.0)
    (`GameplayStatics.OpenLevel` "TopOfNamsan")))

(fn `UserConstructionScript`)
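; Tower crane control panel whose left and right trigger zones rotate a referenced Crane while a character stands in them.
; Both zones start without collision until ActiveButton plays a timeline driving a white overlay material across all static meshes.
; When it finishes, it enables custom depth stencil on the meshes, clears the actor's tags and turns on trigger collision.
; Overlaps start or stop rotation and swap the button lights between blue and red.
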(event `self.ReceiveBeginPlay`
  (`PrimitiveComponent.SetCollisionEnabled` (`self.Right`) "NoCollision")
  (`PrimitiveComponent.SetCollisionEnabled` (`self.Left`) "NoCollision")
  (bind _returnvalue (`KismetMaterialLibrary.CreateDynamicMaterialInstance` "/Game/CableCarMap/Material/M_WhiteOverlay.M_WhiteOverlay"))
  (set `self.OverlayMID` _returnvalue)
  (for _array_element (`self.K2_GetComponentsByClass` "/Script/Engine.StaticMeshComponent")
    (`MeshComponent.SetOverlayMaterial` _array_element (`self.OverlayMID`))))

(event `ActiveButton`
  (bind (_direction `_새_트랙_0`) (`Timeline|타임라인` :!via `PlayFromStart`)
    (:`Update`
      (`MaterialInstanceDynamic.SetScalarParameterValue` (`self.OverlayMID`) "WhiteProgress" `_새_트랙_0`))
    (:`Finished`
      (for _array_element (`self.K2_GetComponentsByClass` "/Script/Engine.StaticMeshComponent")
        (`PrimitiveComponent.SetRenderCustomDepth` _array_element true)
        (`PrimitiveComponent.SetCustomDepthStencilValue` _array_element 2))
      (`KismetArrayLibrary.Array_Clear` (`self.Tags`))
      (`PrimitiveComponent.SetCollisionEnabled` (`self.Right`) "QueryAndPhysics")
      (`PrimitiveComponent.SetCollisionEnabled` (`self.Left`) "QueryAndPhysics"))))

(event `self.Left.OnComponentBeginOverlap`
  (params (OverlappedComponent :type "PrimitiveComponent Object Reference") (OtherActor :type "Actor Object Reference") (OtherComp :type "PrimitiveComponent Object Reference") (OtherBodyIndex :type Integer) (bFromSweep :type Boolean) (SweepResult :type "HitResult Structure (by ref)"))
  ; 크레인 작동 버튼
  (cast `Character` OtherActor)
  (`/Game/LevelDesign/BluePrint/Machine/BP_TowerCrane_1.Rotate Left` (`self.Crane`))
  (`PrimitiveComponent.SetMaterial` (`self.Left Button`) 0 "/Game/LevelDesign/Materials/M_Create/M_BlueLight1.M_BlueLight1"))

(event `self.Left.OnComponentEndOverlap`
  (params (OverlappedComponent :type "PrimitiveComponent Object Reference") (OtherActor :type "Actor Object Reference") (OtherComp :type "PrimitiveComponent Object Reference") (OtherBodyIndex :type Integer))
  ; 크레인 작동 버튼
  (cast `Character` OtherActor)
  (`/Game/LevelDesign/BluePrint/Machine/BP_TowerCrane_1.Rotate Stop` (`self.Crane`))
  (`PrimitiveComponent.SetMaterial` (`self.Left Button`) 0 "/Game/LevelDesign/Materials/M_Create/M_RedLight.M_RedLight"))

(event `self.Right.OnComponentBeginOverlap`
  (params (OverlappedComponent :type "PrimitiveComponent Object Reference") (OtherActor :type "Actor Object Reference") (OtherComp :type "PrimitiveComponent Object Reference") (OtherBodyIndex :type Integer) (bFromSweep :type Boolean) (SweepResult :type "HitResult Structure (by ref)"))
  ; 크레인 작동 버튼
  (cast `Character` OtherActor)
  (`/Game/LevelDesign/BluePrint/Machine/BP_TowerCrane_1.Rotate Right` (`self.Crane`))
  (`PrimitiveComponent.SetMaterial` (`self.Right Button`) 0 "/Game/LevelDesign/Materials/M_Create/M_BlueLight1.M_BlueLight1"))

(event `self.Right.OnComponentEndOverlap`
  (params (OverlappedComponent :type "PrimitiveComponent Object Reference") (OtherActor :type "Actor Object Reference") (OtherComp :type "PrimitiveComponent Object Reference") (OtherBodyIndex :type Integer))
  ; 크레인 작동 버튼
  (cast `Character` OtherActor)
  (`/Game/LevelDesign/BluePrint/Machine/BP_TowerCrane_1.Rotate Stop` (`self.Crane`))
  (`PrimitiveComponent.SetMaterial` (`self.Right Button`) 0 "/Game/LevelDesign/Materials/M_Create/M_RedLight.M_RedLight"))

(fn `CanInteract`
  (params (player :type "Object Object Reference"))
  (returns (ReturnValue :type Boolean))
  (return false))

(fn `UserConstructionScript`)
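; BP_Disappear is an actor that drives a teleport disappear effect through the M_Teleport material parameter collection.
; Each Tick it writes its location to TeleportWorldPosition and samples a float curve into AnimOffset, looping by accumulated time modulo the curve's time range.
; The collection values are shared, so only one instance may run this logic in a world, as the in-graph note warns.
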(event `self.ReceiveTick`
  (params (DeltaSeconds :type "Float (single-precision)"))
  (bind _curve (`self.curve`))
  (bind (_mintime _maxtime) (`CurveBase.GetTimeRange` _curve))
  ; 절대 한 월드에 이 로직이 두개 굴러가게 하면 안돼
  (bind _output_get (set `self.TotalTime` (+ DeltaSeconds (`self.TotalTime`))))
  (`KismetMaterialLibrary.SetVectorParameterValue` "/Game/Teleport/Materials/M_Teleport.M_Teleport" "TeleportWorldPosition" (`KismetMathLibrary.Conv_VectorToLinearColor` (`self.K2_GetActorLocation`)))
  (`KismetMaterialLibrary.SetScalarParameterValue` "/Game/Teleport/Materials/M_Teleport.M_Teleport" "AnimOffset" (`CurveFloat.GetFloatValue` _curve (mod _output_get (- _maxtime _mintime)))))

(fn `UserConstructionScript`)
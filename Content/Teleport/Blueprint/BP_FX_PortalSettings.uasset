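; BP_FX_PortalSettings is an actor that hosts a configurable portal particle effect for teleporting.
; Its construction script assigns the effect template and optionally overrides the base and secondary colour parameters.
; Tick accumulates time and, when Repeat is enabled, calls ResetSystem each time the reset interval elapses.
; ResetSystem restarts the effect and zeroes the timer on the referenced TeleportPositionBP, if valid, restarting both together.
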(event `self.ReceiveBeginPlay`)

(event `self.ReceiveTick`
  (params (DeltaSeconds :type "Float (single-precision)"))
  (bind _output_get (set `self.SumTime` (+ DeltaSeconds (`self.SumTime`))))
  (if (>= _output_get (`self.ResetTime`))
    (if (`self.Repeat`)
      (set `self.SumTime` 0.0)
      (`self.ResetSystem`))))

(fn `ResetSystem`
  (bind _effect (`self.Effect`))
  (bind _teleportpositionbp (`self.teleportPositionBP`))
  (`ActorComponent.Deactivate` _effect)
  (`ActorComponent.Activate` _effect true)
  (if (`KismetSystemLibrary.IsValid` _teleportpositionbp)
    (set `/Game/Teleport/Blueprint/B_FX_TeleportPosition.TotalTime` 0.0 _teleportpositionbp)))

(fn `UserConstructionScript`
  (bind _effect (`self.Effect`))
  (`ParticleSystemComponent.SetTemplate` (`self.Effect`) (`self.EffectTemplate`))
  (if (`self.overwriteColours`)
    (`ParticleSystemComponent.SetColorParameter` _effect "BaseColour" (`self.BaseColour`))
    (`ParticleSystemComponent.SetColorParameter` _effect "Secondcolour" (`self.SecondaryColour`))))